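; Spawner that fills a queue with BP_Person AI running BT_Person, up to the number of points in its linked QuePoint.
; BeginPlay caches that limit; the Spawn event, fired by BP_BBB, compares it to the count of all BP_Person actors.
; While below it, Spawn waits SpawnDelay, spawns at SpawnPoint, passes the queue and disappear point references, increments occupancy, then calls itself again.
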(event Custom|Spawn
  ;[1 0 0] NOTE: This system requires the usage of BP_BBB to fire the spawn event
  ;;[1 1 1] Handles spawning of AI if que points are maxed out
  (bind _outactors (Actor|GetAllActorsOfClass "/Game/AI/BP_Person.BP_Person_C"))
  (if (< (Utilities|Array|Length _outactors) (Variables|Default|GetMaxQuePoints))
    ;;[1 1 1] Spawns AI on target point selected in viewport
    (Utilities|FlowControl|Delay (Variables|Default|GetSpawnDelay))
    (bind _returnvalue (AI|SpawnAIFromClass "/Game/AI/BP_Person.BP_Person_C" "/Game/AI/BT_Person.BT_Person" (Transformation|GetWorldLocation (Variables|/Script/Engine.Actor|GetRootComponent (Variables|Default|GetSpawnPoint))) "0, 0, 0" false 0))
    ;;[1 1 1] Handles references, increasing occupied and looping to spawn enemies
    (Class|BPIAI|SendOverRefs(Message) _returnvalue (Variables|Default|GetQuePoint) (Variables|Default|GetDisappearPoint))
    (Default|IncreaseOccupied (Variables|Default|GetQuePoint))
    (CallFunction|Spawn)))

(event EventBeginPlay
  ;[1 0 0] NOTE: This system requires the usage of BP_BBB to fire the spawn event
  ;;[1 1 1] Sets max que points (don't need to worry about changing the maximum AI que points as long as you set up the que point BP right)
  (Variables|Default|SetMaxQuePoints (Utilities|Array|Length (Variables|/Game/AI/BP_QuePoints.BP_QuePoints_C|GetQuePoints (Variables|Default|GetQuePoint)))))

(fn ConstructionScript)
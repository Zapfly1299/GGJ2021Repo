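; BP_AIReffer is a trigger box that hands the player a reference to the AI person standing inside it.
; On BeginPlay it caches the first person character.
; When a BP_Person overlaps its box, it stores that person, writes it into the player's AI variable and calls the person's InitialText to start their opening text.
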(event OnComponentBeginOverlap(Box)
  (params (OverlappedComponent :type Primitive%20Component%20Object%20Reference) (OtherActor :type Actor%20Object%20Reference) (OtherComp :type Primitive%20Component%20Object%20Reference) (OtherBodyIndex :type Integer) (bFromSweep :type Boolean) (SweepResult :type Hit%20Result%20Structure%20%28by%20ref%29))
  ;[1 1 1] Gets AI ref and gives it to the player and starts initial text of AI who stands in box
  (if (== (Utilities|GetClass OtherActor) "/Game/AI/BP_Person.BP_Person_C")
    (bind _asbp_person (Utilities|Casting|CastToBP_Person OtherActor))
    (bind _output_get (Variables|Default|SetAI _asbp_person))
    (Variables|/Game/Blueprints/FirstPersonCharacter.FirstPersonCharacter_C|SetAI (Variables|Default|GetPlayerRef) _output_get)
    (Default|InitialText _asbp_person)))

(event EventBeginPlay
  ;[1 1 1] Sets ref of player
  (bind _asfirst_person_character (Utilities|Casting|CastToFirstPersonCharacter (Game|Player|GetPlayerPawn 0)))
  (Variables|Default|SetPlayerRef _asfirst_person_character))

(fn ConstructionScript)
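; BP_ItemSpawner spawns BP_Item actors at the positions of randomly picked SpawnLocations actors.
; BeginPlay calls SpawnItem for an initial batch, and SpawnItem also applies a zero-vector impulse to each new item's mesh.
; StartSpawning, not triggered within this file, re-calls itself after a delay, spawning only while the world's BP_Item count is below MaxAllowedItems.
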(event Custom|StartSpawning
  (bind _outactors (Actor|GetAllActorsOfClass "/Game/Blueprints/BP_Item.BP_Item_C"))
  (if (>= (Utilities|Array|Length _outactors) (Variables|Default|GetMaxAllowedItems))
    (Utilities|FlowControl|Delay (Variables|Default|GetDelayBetweenSpawns))
    (CallFunction|StartSpawning)
    (else
      (CallFunction|SpawnItem)
      (Utilities|FlowControl|Delay (Variables|Default|GetDelayBetweenSpawns))
      (CallFunction|StartSpawning))))

(event EventBeginPlay
  (for _index (range 0 (- (Variables|Default|GetInitialItemAmount) 1))
    (CallFunction|SpawnItem)))

(fn ConstructionScript)

(fn SpawnItem
  (bind _returnvalue (Game|SpawnActorfromClass "/Game/Blueprints/BP_Item.BP_Item_C" (Math|Transform|MakeTransform (Transformation|GetActorLocation (Utilities|Array|Get(acopy) (Variables|Default|GetSpawnLocations) (Math|Random|RandomIntegerinRange 0 (Utilities|Array|LastIndex (Variables|Default|GetSpawnLocations))))) "0, 0, 0" "1,1,1") "Undefined" 0 0))
  (Physics|AddImpulse (Variables|/Game/Blueprints/BP_Item.BP_Item_C|GetItemMesh _returnvalue) "0, 0, 0" "None" false))
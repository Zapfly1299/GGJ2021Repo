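; Test AI actor for a lost-property customer that asks for an item with Correct, Missing Information or Wrong information.
; On BeginPlay it rolls a person type from chance ranges, then takes a random item from the game instance's AI choices.
; It indexes DT_Convo rows by that type; Wrong people also gather final-choice lines and a lost item not already existing.
; ConversationStarter prints a random line formatted with item details, currently only for Correct and Missing Information.
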(event Custom|Break
  (Utilities|Array|ForEachLoopwithBreak (Variables|Default|GetPersonChances)) ; enters at Break
)

(event Custom|AssignItem
  (bind _lostitemsrows (Variables|Default|GetLostItemsRows))
  (bind _instanceref (Variables|Default|GetInstanceRef))
  (bind _aichoices (Variables|/Game/Blueprints/GI_Main.GI_Main_C|GetAIChoices _instanceref))
  (bind _output (Utilities|Array|Get(acopy) _aichoices))
  (Utilities|Array|Shuffle (Variables|/Game/Blueprints/GI_Main.GI_Main_C|GetAIChoices (Variables|Default|GetInstanceRef)))
  (Variables|Default|SetDesiredItem _output)
  (Utilities|Array|RemoveItem _aichoices _output)
  (Variables|Default|SetItem%20Name (.ItemName (Utilities|Struct|BreakS_ItemInformation (.ItemInformation (Utilities|Struct|BreakS_SavedItem (Variables|Default|GetDesiredItem))))))
  (Variables|Default|SetColour (.Colour (Utilities|Struct|BreakS_ItemInformation (.ItemInformation (Utilities|Struct|BreakS_SavedItem (Variables|Default|GetDesiredItem))))))
  (Variables|Default|SetSize (.Size (Utilities|Struct|BreakS_SavedItem (Variables|Default|GetDesiredItem))))
  (switch Utilities|FlowControl|Switch|SwitchonE_PersonType (Variables|Default|GetPersonType)
    (:NewEnumerator0
      (CallFunction|GetConversationType))
    (:NewEnumerator1
      (CallFunction|GetConversationType))
    (:NewEnumerator2
      (CallFunction|GetConversationType)
      (|GetFinalTexts
        (:Out
          (for _array_element (Variables|/Game/Blueprints/GI_Main.GI_Main_C|GetExistingItems (Variables|Default|GetInstanceRef))
            (Utilities|Array|RemoveItem (Variables|Default|GetLostItemsRows) (.RowName (Utilities|Struct|BreakS_SavedItem _array_element))))
          (Utilities|Array|Shuffle _lostitemsrows)
          (bind _returnvalue (Utilities|GetDataTableRow "/Game/Blueprints/DT_LostItems.DT_LostItems" (Utilities|Array|Get(acopy) _lostitemsrows))
            (:then
              (Variables|Default|SetWrongItem _returnvalue))))))))

(event Custom|ConversationStarter
  (switch Utilities|FlowControl|Switch|SwitchonE_PersonType (Variables|Default|GetPersonType)
    (:NewEnumerator0
      (bind _result (CallFunction|GetText (Variables|Default|GetConvoRowNames)))
      (Development|PrintText _result))
    (:NewEnumerator1
      ;[1 1 1] Need to make it so missing info and wrong require more interactions
      (bind _result_2 (CallFunction|GetText (Variables|Default|GetConvoRowNames)))
      (Development|PrintText _result_2))))

(event EventBeginPlay
  (bind _asgi_main (Utilities|Casting|CastToGI_Main (Game|GetGameInstance)))
  (Variables|Default|SetInstanceRef _asgi_main)
  (bind _outrownames (DataTable|GetDataTableRowNames "/Game/Blueprints/DT_Convo.DT_Convo"))
  (Variables|Default|SetConvoRowNames _outrownames)
  (bind _outrownames_2 (DataTable|GetDataTableRowNames "/Game/Blueprints/DT_LostItems.DT_LostItems"))
  (Variables|Default|SetLostItemsRows _outrownames_2)
  (Variables|Default|SetRandomInt (Math|Random|RandomIntegerinRange 1 100))
  (bind _array_element (Utilities|Array|ForEachLoopwithBreak (Variables|Default|GetPersonChances))
    (:LoopBody
      (if (CallFunction|CheckChances (.LowerChance (Utilities|Struct|BreakS_PersonChance _array_element)) (.UpperChance (Utilities|Struct|BreakS_PersonChance _array_element)) (Variables|Default|GetRandomInt))
        (Variables|Default|SetPersonType (.PersonType (Utilities|Struct|BreakS_PersonChance _array_element)))
        (CallFunction|Break)))
    (:Completed
      (CallFunction|AssignItem))))

(fn ConstructionScript)

(fn CheckChances
  (params (LowerChance :type Integer) (UpperChance :type Integer) (RandomNumber :type Integer))
  (return (and (>= RandomNumber LowerChance) (<= RandomNumber UpperChance))))

(fn GetConversationType
  (for (_array_element _array_index) (Variables|Default|GetConvoRowNames)
    (bind _returnvalue (Utilities|GetDataTableRow "/Game/Blueprints/DT_Convo.DT_Convo" _array_element)
      (:then
        (if (Utilities|Enum|Equal(Enum) (.ConversationType (Utilities|Struct|BreakS_Conversation _returnvalue)) (Variables|Default|GetPersonType))
          (Utilities|Array|Add (Variables|Default|GetIndexArray) _array_index))))))

(fn RandomIndex
  (params (TargetArray :type Array%20of%20Integers))
  (bind _output_get (Variables|Default|SetIndex (Utilities|Array|Get(acopy) TargetArray (Math|Random|RandomIntegerinRange 0 (Utilities|Array|LastIndex TargetArray)))))
  (return _output_get))

(fn GetText
  (params (Array :type Array%20of%20Names))
  (bind _returnvalue (Utilities|GetDataTableRow "/Game/Blueprints/DT_Convo.DT_Convo" (Utilities|Array|Get(acopy) Array (CallFunction|RandomIndex (Variables|Default|GetIndexArray))))
    (:then
      (Utilities|Array|RemoveIndex Array (Variables|Default|GetIndex))
      (return (Utilities|Text|FormatText (.MainFormatText (Utilities|Struct|BreakS_Conversation _returnvalue)) (Variables|Default|GetItem%20Name) (Variables|Default|GetColour) (Variables|Default|GetSize))))))
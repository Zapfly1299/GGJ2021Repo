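; ScenerySpawner is an actor that spawns random mountain scenery at preset spawn points.
; On BeginPlay it caches the child components of MountainSpawns and TreeSpawns as spawn point arrays.
; SpawnMountain spawns a random actor class from MountainMeshes at a random mountain point's world transform, with no caller in this graph.
; The tree points are gathered, but nothing here spawns at them.
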(event Custom|SpawnMountain
  (bind _mountainspawnsarray (Variables|Default|GetMountainSpawnsArray))
  (bind _mountainmeshes (Variables|Default|GetMountainMeshes))
  (Game|SpawnActorfromClass (Utilities|Array|Get(acopy) _mountainmeshes (- (Math|Random|RandomIntegerinRange 1 (Utilities|Array|Length _mountainmeshes)) 1)) (Transformation|GetWorldTransform (Utilities|Array|Get(acopy) _mountainspawnsarray (- (Math|Random|RandomIntegerinRange 1 (Utilities|Array|Length _mountainspawnsarray)) 1))) "Undefined" 0 0))

(event EventBeginPlay
  (Variables|Default|SetMountainSpawnsArray (Components|GetChildrenComponents (Variables|Default|GetMountainSpawns) false))
  (Variables|Default|SetTreeSpawnsArray (Components|GetChildrenComponents (Variables|Default|GetTreeSpawns) false)))

(fn ConstructionScript)
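; Lost-item actor that takes on a random, not-yet-used identity from DT_LostItems when it spawns.
; BeginPlay filters out rows already in GI_Main's ExistingItems, then ChooseItem shuffles the rest and applies the first row's mesh and material.
; It records the item in ExistingItems and AIChoices, with GetSize randomly rolling small or large and rescaling the mesh per call.
; Delete removes the ExistingItems entry and destroys the actor.
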(event Custom|Delete
  (Utilities|Array|RemoveItem (Variables|/Game/Blueprints/GI_Main.GI_Main_C|GetExistingItems (Variables|Default|GetInstanceRef)) (Utilities|Struct|MakeS_SavedItem (Variables|Default|GetSelectedRow) (Variables|Default|GetSelectedItem) (Variables|Default|GetChosenSize)))
  (Actor|DestroyActor))

(event Custom|ChooseItem
  (bind _instanceref (Variables|Default|GetInstanceRef))
  (Utilities|Array|Shuffle (Variables|Default|GetRowNames))
  (bind _output_get (Variables|Default|SetSelectedRow (Utilities|Array|Get(acopy) (Variables|Default|GetRowNames))))
  (bind _returnvalue (Utilities|GetDataTableRow "/Game/Blueprints/DT_LostItems.DT_LostItems" _output_get)
    (:then
      (bind _output_get_2 (Variables|Default|SetSelectedItem _returnvalue))
      (Components|StaticMesh|SetStaticMesh (Variables|Default|GetItemMesh) (.Mesh (Utilities|Struct|BreakS_ItemInfo _output_get_2)))
      (Rendering|Material|SetMaterial (Variables|Default|GetItemMesh) 0 (.ColourMats (Utilities|Struct|BreakS_ItemInfo _output_get_2)))
      (Utilities|Array|Add (Variables|/Game/Blueprints/GI_Main.GI_Main_C|GetExistingItems _instanceref) (Utilities|Struct|MakeS_SavedItem (Variables|Default|GetSelectedRow) (Variables|Default|GetSelectedItem) (CallFunction|GetSize)))
      (Utilities|Array|Add (Variables|/Game/Blueprints/GI_Main.GI_Main_C|GetAIChoices _instanceref) (Utilities|Struct|MakeS_SavedItem (Variables|Default|GetSelectedRow) (Variables|Default|GetSelectedItem) (CallFunction|GetSize))))))

(event EventBeginPlay
  (bind _outrownames (DataTable|GetDataTableRowNames "/Game/Blueprints/DT_LostItems.DT_LostItems"))
  (Variables|Default|SetRowNames _outrownames)
  (bind _asfirst_person_character (Utilities|Casting|CastToFirstPersonCharacter (Game|Player|GetPlayerPawn 0)))
  (Variables|Default|SetPlayerRef _asfirst_person_character)
  (bind _asgi_main (Utilities|Casting|CastToGI_Main (Game|GetGameInstance)))
  (bind _output_get (Variables|Default|SetInstanceRef _asgi_main))
  (if (Utilities|Array|IsValidIndex (Variables|/Game/Blueprints/GI_Main.GI_Main_C|GetExistingItems _output_get))
    (for _array_element (Variables|/Game/Blueprints/GI_Main.GI_Main_C|GetExistingItems (Variables|Default|GetInstanceRef))
      (Utilities|Array|RemoveItem (Variables|Default|GetRowNames) (.RowName (Utilities|Struct|BreakS_SavedItem _array_element)))))
  (CallFunction|ChooseItem))

(fn ConstructionScript)

(fn GetSize
  (if (>= (Math|Random|RandomIntegerinRange 1 100) 60)
    (Variables|Default|SetChosenSize "large")
    (Transformation|SetWorldScale3D (Variables|Default|GetItemMesh) "1.500000,1.500000,1.500000")
    (else
      (Variables|Default|SetChosenSize "small")
      (Transformation|SetWorldScale3D (Variables|Default|GetItemMesh) "1.000000,1.000000,1.000000")))
  (return (Variables|Default|GetChosenSize)))
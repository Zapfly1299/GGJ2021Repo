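; Test AI person who requests an item through templated dialogue and judges the item brought to it.
; BeginPlay rolls a Correct, Missing Information or Wrong type, picks its conversation DataTable and claims a random item from GI_Main's pool.
; Dialogue is formatted with item details; Wrong types first describe a different item.
; An overlap-gated Interact compares item rows, destroying the player when chances run out; retry text is fetched but not printed.
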(event OnComponentBeginOverlap(Cube)
  (params (OverlappedComponent :type Primitive%20Component%20Object%20Reference) (OtherActor :type Actor%20Object%20Reference) (OtherComp :type Primitive%20Component%20Object%20Reference) (OtherBodyIndex :type Integer) (bFromSweep :type Boolean) (SweepResult :type Hit%20Result%20Structure%20%28by%20ref%29))
  ;[1 1 1] Make this so it only works if player is holding item
  (if (Actor|ActorHasTag OtherActor "Interactable")
    (Variables|Default|SetOverlappedActor OtherActor)
    (Input|EnableInput (Game|GetPlayerController 0))
    (Utilities|FlowControl|Gate true) ; enters at Open
  ))

(event OnComponentEndOverlap(Cube)
  (params (OverlappedComponent :type Primitive%20Component%20Object%20Reference) (OtherActor :type Actor%20Object%20Reference) (OtherComp :type Primitive%20Component%20Object%20Reference) (OtherBodyIndex :type Integer))
  ;[1 1 1] Make this so it only works if player is holding item
  (if (Actor|ActorHasTag OtherActor "Interactable")
    (Variables|Default|SetOverlappedActor 0)
    (Input|DisableInput (Game|GetPlayerController 0))
    (Utilities|FlowControl|Gate true) ; enters at Close
  ))

(event Custom|Break
  (Utilities|Array|ForEachLoopwithBreak (Variables|Default|GetPersonChances)) ; enters at Break
)

(event Custom|AssignItem
  (bind _instanceref (Variables|Default|GetInstanceRef))
  (bind _instanceref_2 (Variables|Default|GetInstanceRef))
  (bind _aichoices (Variables|/Game/Blueprints/GI_Main.GI_Main_C|GetAIChoices _instanceref_2))
  (bind _aichoices_2 (Variables|/Game/Blueprints/GI_Main.GI_Main_C|GetAIChoices _instanceref))
  (bind _output (Utilities|Array|Get(acopy) _aichoices))
  (Utilities|Array|Shuffle (Variables|/Game/Blueprints/GI_Main.GI_Main_C|GetAIChoices (Variables|Default|GetInstanceRef)))
  (Variables|Default|SetDesiredItem _output)
  (Utilities|Array|RemoveItem _aichoices _output)
  (Variables|Default|SetItem%20Name (.ItemName (Utilities|Struct|BreakS_ItemInfo (.ItemInformation (Utilities|Struct|BreakS_SavedItem (Variables|Default|GetDesiredItem))))))
  (Variables|Default|SetColour (.Colour (Utilities|Struct|BreakS_ItemInfo (.ItemInformation (Utilities|Struct|BreakS_SavedItem (Variables|Default|GetDesiredItem))))))
  (Variables|Default|SetSize (.Size (Utilities|Struct|BreakS_SavedItem (Variables|Default|GetDesiredItem))))
  (switch Utilities|FlowControl|Switch|SwitchonE_PersonType (Variables|Default|GetPersonType)
    (:NewEnumerator0
      (CallFunction|GetConversationType :!label _label))
    (:NewEnumerator1
      (goto _label))
    (:NewEnumerator2
      (CallFunction|GetConversationType)
      (Utilities|Array|Shuffle _aichoices_2)
      (Variables|Default|SetWrongItem (Utilities|Array|Get(acopy) _aichoices_2))))
  (bind _result (CallFunction|GetText))
  (Development|PrintText _result true true "(R=0.000000,G=0.660000,B=1.000000,A=1.000000)" 5e+01))

(event EventBeginPlay
  (bind _asgi_main (Utilities|Casting|CastToGI_Main (Game|GetGameInstance)))
  (Variables|Default|SetInstanceRef _asgi_main)
  (Variables|Default|SetRandomInt (Math|Random|RandomIntegerinRange 1 100))
  (bind _array_element (Utilities|Array|ForEachLoopwithBreak (Variables|Default|GetPersonChances))
    (:LoopBody
      (if (CallFunction|CheckChances (.LowerChance (Utilities|Struct|BreakS_PersonChance _array_element)) (.UpperChance (Utilities|Struct|BreakS_PersonChance _array_element)) (Variables|Default|GetRandomInt))
        (bind _output_get (Variables|Default|SetPersonType (.PersonType (Utilities|Struct|BreakS_PersonChance _array_element))))
        (switch Utilities|FlowControl|Switch|SwitchonE_PersonType _output_get
          (:NewEnumerator0
            (Variables|Default|SetConversationTable "/Game/Blueprints/DT_CorrectPerson.DT_CorrectPerson"))
          (:NewEnumerator1
            (Variables|Default|SetConversationTable "/Game/Blueprints/DT_MissingInfo.DT_MissingInfo"))
          (:NewEnumerator2
            (Variables|Default|SetConversationTable "/Game/Blueprints/DT_WrongPerson.DT_WrongPerson")))
        (bind _outrownames (DataTable|GetDataTableRowNames (Variables|Default|GetConversationTable)))
        (Variables|Default|SetConvoRowNames _outrownames)))
    (:Completed
      (CallFunction|AssignItem))))

(event EventInteracted
  (params (Item :type BP%20Item%20Object%20Reference))
  (if (Utilities|Name|Equal(Name) (Variables|/Game/Blueprints/BP_Item.BP_Item_C|GetSelectedRow Item) (.RowName (Utilities|Struct|BreakS_SavedItem (Variables|Default|GetDesiredItem))))
    (Development|PrintText "CORRECT")
    (else
      (Math|Integer|IncrementInt (Variables|Default|GetTimesInteracted)
        (:%20%20
          (if (== (Variables|Default|GetTimesInteracted) (Variables|Default|GetNoOfChances))
            (Development|PrintText (Utilities|Struct|BreakS_Convo (Variables|Default|GetDesiredText)))
            (bind _asfirst_person_character (Utilities|Casting|CastToFirstPersonCharacter (Game|Player|GetPlayerPawn 0)))
            (Actor|DestroyActor _asfirst_person_character)
            (else
              (CallFunction|GetText))))))))

(event Input|ActionEvents|InputActionInteract
  (params (Key :type Key%20Structure :default "None"))
  ;[1 1 1] Make this so it only works if player is holding item
  (:Pressed
    (Utilities|FlowControl|Gate true
      (:Exit
        (bind _asbp_item (Utilities|Casting|CastToBP_Item (Variables|Default|GetOverlappedActor)))
        (CallFunction|Interacted _asbp_item)))))

(fn ConstructionScript)

(fn CheckChances
  (params (LowerChance :type Integer) (UpperChance :type Integer) (RandomNumber :type Integer))
  (return (and (>= RandomNumber LowerChance) (<= RandomNumber UpperChance))))

(fn GetConversationType
  (Utilities|Array|Shuffle (Variables|Default|GetConvoRowNames))
  (bind _returnvalue (Utilities|GetDataTableRow (Variables|Default|GetConversationTable) (Utilities|Array|Get(acopy) (Variables|Default|GetConvoRowNames)))
    (:then
      (bind _output_get (Variables|Default|SetDesiredText _returnvalue))
      (Variables|Default|SetNoOfChances (.noofchances _output_get)))))

(fn GetText
  (bind _wrongitem (Variables|Default|GetWrongItem))
  (bind _desiredtext (Variables|Default|GetDesiredText))
  (bind (_noofchances _interact1 _interact2 _interact3) (Utilities|Struct|BreakS_Convo _desiredtext))
  (bind (_rowname _iteminformation _size) (Utilities|Struct|BreakS_SavedItem _wrongitem))
  (bind (_itemname _colour) (Utilities|Struct|BreakS_ItemInfo _iteminformation))
  (switch int (Variables|Default|GetTimesInteracted)
    (:0
      (Variables|Default|SetFormatText _interact1)
      (switch Utilities|FlowControl|Switch|SwitchonE_PersonType (Variables|Default|GetPersonType)
        (:NewEnumerator0
          _)
        (:NewEnumerator1
          _)
        (:NewEnumerator2
          (return (Utilities|Text|FormatText (Variables|Default|GetFormatText) _itemname _colour _size)))))
    (:1
      (Variables|Default|SetFormatText _interact2))
    (:2
      (Variables|Default|SetFormatText _interact3)))
  (return (Utilities|Text|FormatText (Variables|Default|GetFormatText) (Variables|Default|GetItem%20Name) (Variables|Default|GetColour) (Variables|Default|GetSize))))
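; BP_QuePoints is an AI queue Blueprint that tracks how many of its queue points are occupied.
; IncreaseOccupied increments OccupiedPlaces and compares it to the QuePoints array length, but the over-capacity branch does nothing.
; DecreaseOccupied decrements the counter and resets it to zero only if it is already negative, so it can reach minus one.
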(event Custom|IncreaseOccupied
  (bind _result (Math|Integer|IncrementInt (Variables|Default|GetOccupiedPlaces))
    (:%20%20
      (if (> _result (Utilities|Array|Length (Variables|Default|GetQuePoints)))
        _))))

(event Custom|DecreaseOccupied
  (Variables|Default|SetOccupiedPlaces (select (< (Variables|Default|GetOccupiedPlaces) 0) (Class|KismetSystemLibrary|MakeLiteralInteger) (- (Variables|Default|GetOccupiedPlaces) 1))))

(fn ConstructionScript)
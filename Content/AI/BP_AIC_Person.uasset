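; AI controller for a person character that starts the BT_Person behavior tree on BeginPlay and stores its controlled pawn.
; Any AI perception update, noted as a noise made somewhere, sets the NextPoint blackboard bool to true without checking the stimulus.
; A placeholder-named custom event, Ooooooo, prints a debug message and sets the AtFrontOfQue blackboard bool to true.
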(event OnTargetPerceptionUpdated(AIPerception)
  (params (Actor :type Actor%20Object%20Reference) (Stimulus :type AI%20Stimulus%20Structure))
  ;[1 1 1] Just needs a noise made somehwere
  (AI|Components|Blackboard|SetValueasBool (AI|GetBlackboard 0) (Utilities|Name|MakeLiteralName "NextPoint") true))

(event Custom|Ooooooo
  (Development|PrintString "Hello")
  (AI|Components|Blackboard|SetValueasBool (AI|GetBlackboard 0) (Utilities|Name|MakeLiteralName "AtFrontOfQue") true))

(event EventBeginPlay
  (AI|RunBehaviorTree "/Game/AI/BT_Person.BT_Person")
  (Variables|Default|SetControlledPawn (Pawn|GetControlledPawn)))

(fn ConstructionScript)
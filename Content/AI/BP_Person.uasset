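; BP_Person is an AI customer who requests an item from the player through dialogue.
; It rolls a weighted person type, drawing dialogue from that type's data table and an item from GI_Main's pool.
; Wrong types first describe another item, then the real one on retries.
; Correct delivery succeeds; exhausted chances or patience fail, each updating the game mode's score and time and reporting a noise event after a delay.
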(event OnComponentBeginOverlap(Box)
  (params (OverlappedComponent :type Primitive%20Component%20Object%20Reference) (OtherActor :type Actor%20Object%20Reference) (OtherComp :type Primitive%20Component%20Object%20Reference) (OtherBodyIndex :type Integer) (bFromSweep :type Boolean) (SweepResult :type Hit%20Result%20Structure%20%28by%20ref%29))
  (bind _playerref (Variables|Default|GetPlayerRef))
  (bind _pickedupitem (Variables|/Game/Blueprints/FirstPersonCharacter.FirstPersonCharacter_C|GetPickedUpItem _playerref))
  ;[1 1 1] Handles overlapping of item, allows player to interact with AI
  (Utilities|IsValid _pickedupitem
    (:Is%20Valid
      (if (Math|Boolean|ANDBoolean (== _pickedupitem OtherActor) (Actor|ActorHasTag OtherActor "Interactable") (Variables|Default|GetAcceptingItem))
        (Variables|/Game/Blueprints/FirstPersonCharacter.FirstPersonCharacter_C|SetCanInteract (Variables|Default|GetPlayerRef) true)))))

(event OnComponentEndOverlap(Box)
  (params (OverlappedComponent :type Primitive%20Component%20Object%20Reference) (OtherActor :type Actor%20Object%20Reference) (OtherComp :type Primitive%20Component%20Object%20Reference) (OtherBodyIndex :type Integer))
  (bind _playerref (Variables|Default|GetPlayerRef))
  (bind _pickedupitem (Variables|/Game/Blueprints/FirstPersonCharacter.FirstPersonCharacter_C|GetPickedUpItem _playerref))
  ;[1 1 1] Handles overlapping of item, allows player to interact with AI
  (Utilities|IsValid _pickedupitem
    (:Is%20Valid
      (if (and (== _pickedupitem OtherActor) (Actor|ActorHasTag OtherActor "Interactable"))
        (Variables|/Game/Blueprints/FirstPersonCharacter.FirstPersonCharacter_C|SetCanInteract (Variables|Default|GetPlayerRef) false)))))

(event Custom|Break
  ;[1 1 1] Gets random integer and checks against chances to see which person type the AI needs to be (person chances customisable in person chances variable)
  (Utilities|Array|ForEachLoopwithBreak (Variables|Default|GetPersonChances)) ; enters at Break
)

(event Custom|AssignItem
  (bind _instanceref (Variables|Default|GetInstanceRef))
  (bind _instanceref_2 (Variables|Default|GetInstanceRef))
  (bind _aichoices (Variables|/Game/Blueprints/GI_Main.GI_Main_C|GetAIChoices _instanceref_2))
  (bind _aichoices_2 (Variables|/Game/Blueprints/GI_Main.GI_Main_C|GetAIChoices _instanceref))
  (bind _output (Utilities|Array|Get(acopy) _aichoices))
  ;[1 1 1] Decides on which item AI desires and then sets variables needed for formatting
  (Utilities|Array|Shuffle (Variables|/Game/Blueprints/GI_Main.GI_Main_C|GetAIChoices (Variables|Default|GetInstanceRef)))
  (Variables|Default|SetDesiredItem _output)
  (Utilities|Array|RemoveItem _aichoices _output)
  (Variables|Default|SetItem%20Name (.ItemName (Utilities|Struct|BreakS_ItemInfo (.ItemInformation (Utilities|Struct|BreakS_SavedItem (Variables|Default|GetDesiredItem))))))
  (Variables|Default|SetColour (.Colour (Utilities|Struct|BreakS_ItemInfo (.ItemInformation (Utilities|Struct|BreakS_SavedItem (Variables|Default|GetDesiredItem))))))
  (Variables|Default|SetSize (.Size (Utilities|Struct|BreakS_SavedItem (Variables|Default|GetDesiredItem))))
  ;[1 1 1] Gets conversation type depending on person type, has different end functionality for wrong person type
  (switch Utilities|FlowControl|Switch|SwitchonE_PersonType (Variables|Default|GetPersonType)
    (:NewEnumerator0
      (CallFunction|GetConversationType :!label _label))
    (:NewEnumerator1
      (goto _label))
    (:NewEnumerator2
      (CallFunction|GetConversationType)
      (Utilities|Array|Shuffle _aichoices_2)
      (Variables|Default|SetWrongItem (Utilities|Array|Get(acopy) _aichoices_2)))))

(event Custom|InitialText
  ;[1 1 1] Start initial text
  (Utilities|FlowControl|DoOnce false
    (:Completed
      (Variables|/Script/Engine.PrimitiveComponent|SetbGenerateOverlapEvents (Variables|Default|GetBox) true)
      (bind _result (CallFunction|GetText))
      (Default|WriteText (Variables|Default|GetDialogueRef) _result)
      ;[1 1 1] Patience timer
      (Utilities|Time|SetTimerbyEvent (delegate Custom|PatienceTimer) 1.0 true))))

(event Custom|The%20First%20Boi
  (bind _asbp_aic_person (Utilities|Casting|CastToBP_AIC_Person (Pawn|GetController)))
  (Default|Ooooooo _asbp_aic_person))

(event Custom|PatienceTimer
  ;[1 1 1] Patience timer
  (bind _result (Math|Float|IncrementFloat (Variables|Default|GetPatienceTime))
    (:%20%20
      (if (== _result (Variables|Default|GetPatienceTolerance))
        (CallFunction|Fail)))))

(event Custom|Fail
  ;[1 1 1] Handles fail logic
  (Variables|Default|SetAcceptingItem false)
  (Components|DestroyComponent (Variables|Default|GetBox))
  (Default|WriteText (Variables|Default|GetDialogueRef) (Utilities|Struct|BreakS_Convo (Variables|Default|GetDesiredText)))
  (Utilities|Array|Add (Variables|/Game/Blueprints/GI_Main.GI_Main_C|GetAIChoices (Variables|Default|GetInstanceRef)) (Variables|Default|GetDesiredItem))
  (Default|PeopleFail (.AsFirst%20Person%20Game%20Mode (Utilities|Casting|CastToFirstPersonGameMode (Game|GetGameMode))))
  (Utilities|FlowControl|Delay 3.0)
  (Class|AISenseHearing|ReportNoiseEvent (Transformation|GetActorLocation) 1.0 self 0.0 "None")
  (Default|DecreaseTime (.AsFirst%20Person%20Game%20Mode (Utilities|Casting|CastToFirstPersonGameMode (Game|GetGameMode))) (Variables|Default|GetDecreaseAmount)))

(event Custom|Succeed
  ;[1 1 1] Handles success logic
  (Variables|Default|SetAcceptingItem false)
  (Components|DestroyComponent (Variables|Default|GetBox))
  (Default|WriteText (Variables|Default|GetDialogueRef) (Utilities|Struct|BreakS_Convo (Variables|Default|GetDesiredText)))
  (Default|PeopleSuccess (.AsFirst%20Person%20Game%20Mode (Utilities|Casting|CastToFirstPersonGameMode (Game|GetGameMode))))
  (Default|Delete (Variables|Default|GetInteractedItem))
  (Default|StartSpawning (Variables|Default|GetItemSpawner))
  (Utilities|FlowControl|Delay 3.0)
  (Class|AISenseHearing|ReportNoiseEvent (Transformation|GetActorLocation) 1.0 self 0.0 "None")
  (Default|IncreaseTime (.AsFirst%20Person%20Game%20Mode (Utilities|Casting|CastToFirstPersonGameMode (Game|GetGameMode))) (Variables|Default|GetIncreaseAmount)))

(event EventBeginPlay
  ;[1 1 1] Reference shit on begin play
  (bind _asgi_main (Utilities|Casting|CastToGI_Main (Game|GetGameInstance)))
  (Variables|Default|SetInstanceRef _asgi_main)
  (bind _asfirst_person_character (Utilities|Casting|CastToFirstPersonCharacter (Game|Player|GetPlayerPawn 0)))
  (bind _output_get (Variables|Default|SetPlayerRef _asfirst_person_character))
  (Variables|Default|SetDialogueRef (Variables|/Game/Blueprints/FirstPersonCharacter.FirstPersonCharacter_C|GetDialogueWidget _output_get))
  ;[1 1 1] Gets random integer and checks against chances to see which person type the AI needs to be (person chances customisable in person chances variable)
  (Variables|Default|SetRandomInt (Math|Random|RandomIntegerinRange 1 100))
  (bind _array_element (Utilities|Array|ForEachLoopwithBreak (Variables|Default|GetPersonChances))
    (:LoopBody
      (if (CallFunction|CheckChances (.LowerChance (Utilities|Struct|BreakS_PersonChance _array_element)) (.UpperChance (Utilities|Struct|BreakS_PersonChance _array_element)) (Variables|Default|GetRandomInt))
        ;[1 1 1] Data table management, decides which data table is needed dependant on person type
        (bind _output_get_2 (Variables|Default|SetPersonType (.PersonType (Utilities|Struct|BreakS_PersonChance _array_element))))
        (switch Utilities|FlowControl|Switch|SwitchonE_PersonType _output_get_2
          (:NewEnumerator0
            (Variables|Default|SetConversationTable "/Game/Blueprints/DT_CorrectPerson.DT_CorrectPerson"))
          (:NewEnumerator1
            (Variables|Default|SetConversationTable "/Game/Blueprints/DT_MissingInfo.DT_MissingInfo"))
          (:NewEnumerator2
            (Variables|Default|SetConversationTable "/Game/Blueprints/DT_WrongPerson.DT_WrongPerson")))
        (bind _outrownames (DataTable|GetDataTableRowNames (Variables|Default|GetConversationTable)))
        (Variables|Default|SetConvoRowNames _outrownames)))
    (:Completed
      ;[1 1 1] Calls assign item
      (CallFunction|AssignItem))))

(event EventSendOverRefs
  (params (QuePoint :type BP%20Que%20Points%20Object%20Reference) (DisappearPoint :type BP%20Disappear%20Point%20Object%20Reference) (ItemSpawner :type BP%20Item%20Spawner%20Object%20Reference))
  (Variables|Default|SetQuePoints QuePoint)
  (Variables|Default|SetDisappearPoint DisappearPoint)
  (Variables|Default|SetItemSpawner ItemSpawner))

(event EventKillSelf
  (Actor|DestroyActor))

(event EventInteracted
  (params (Item :type BP%20Item%20Object%20Reference))
  ;[1 1 1] Handles interaction with the item
  (Variables|Default|SetInteractedItem Item)
  (if (Utilities|Name|Equal(Name) (Variables|/Game/Blueprints/BP_Item.BP_Item_C|GetSelectedRow Item) (.RowName (Utilities|Struct|BreakS_SavedItem (Variables|Default|GetDesiredItem))))
    (CallFunction|Succeed)
    (else
      (Math|Integer|IncrementInt (Variables|Default|GetTimesInteracted)
        (:%20%20
          (if (== (Variables|Default|GetTimesInteracted) (Variables|Default|GetNoOfChances))
            (CallFunction|Fail)
            (else
              (bind _result (CallFunction|GetText))
              (Default|WriteText (Variables|Default|GetDialogueRef) _result))))))))

(fn ConstructionScript)

(fn CheckChances
  (params (LowerChance :type Integer) (UpperChance :type Integer) (RandomNumber :type Integer))
  (return (and (>= RandomNumber LowerChance) (<= RandomNumber UpperChance))))

(fn GetConversationType
  ;[1 1 1] Gets a random interaction conversation depending on which type of person it is
  (Utilities|Array|Shuffle (Variables|Default|GetConvoRowNames))
  (bind _returnvalue (Utilities|GetDataTableRow (Variables|Default|GetConversationTable) (Utilities|Array|Get(acopy) (Variables|Default|GetConvoRowNames)))
    (:then
      (bind _output_get (Variables|Default|SetDesiredText _returnvalue))
      (Variables|Default|SetNoOfChances (.noofchances _output_get)))))

(fn GetText
  (bind _wrongitem (Variables|Default|GetWrongItem))
  (bind _desiredtext (Variables|Default|GetDesiredText))
  (bind (_noofchances _interact1 _interact2 _interact3) (Utilities|Struct|BreakS_Convo _desiredtext))
  (bind (_rowname _iteminformation _size) (Utilities|Struct|BreakS_SavedItem _wrongitem))
  (bind (_itemname _colour) (Utilities|Struct|BreakS_ItemInfo _iteminformation))
  ;[1 1 1] Text formatting and gets wrong item for the wrong person type of conversation
  (switch int (Variables|Default|GetTimesInteracted)
    (:0
      (Variables|Default|SetFormatText _interact1)
      (switch Utilities|FlowControl|Switch|SwitchonE_PersonType (Variables|Default|GetPersonType)
        (:NewEnumerator0
          _)
        (:NewEnumerator1
          _)
        (:NewEnumerator2
          (return (Utilities|Text|FormatText (Variables|Default|GetFormatText) _itemname _colour _size)))))
    (:1
      (Variables|Default|SetFormatText _interact2))
    (:2
      (Variables|Default|SetFormatText _interact3)))
  (return (Utilities|Text|FormatText (Variables|Default|GetFormatText) (Variables|Default|GetItem%20Name) (Variables|Default|GetColour) (Variables|Default|GetSize))))